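; Character creator preview actor that shows a customizable character and opens the creator UI and pause menu.
; BeginPlay wires body, hair, eye and clothing meshes into BPCCharacterCustomization, starts four async Mutable mesh updates and makes the parts follow the body's pose.
; Input drives an orbit and zoom camera with head close-up and full-body presets.
; Tick applies rotation, head tracking and a height-slider vertical mesh offset.
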(event Custom|OnInitialUpdateFinished
  (params (Result :type Update%20Context%20Structure%20%28by%20ref%29))
  (Default|OnMeshUpdateFinished (Variables|Default|GetBPC_CharacterCustomization) Result))

(event EventBeginPlay
  (bind _returnvalue (Game|GetPlayerController 0))
  (bind _bpc_charactercustomization (Variables|Default|GetBPC_CharacterCustomization))
  (bind _customizableskeletal (Variables|Default|GetCustomizableSkeletal))
  (bind _bpc_charactercustomization_2 (Variables|Default|GetBPC_CharacterCustomization))
  (bind _clothingmeshes (Variables|/Game/Blueprints/BPC_CharacterCustomization.BPC_CharacterCustomization_C|GetClothingMeshes _bpc_charactercustomization_2))
  (Input|SetInputModeGameandUI (Game|GetPlayerController 0) 0 "DoNotLock" false false)
  (Variables|/Game/Blueprints/BPC_CharacterCustomization.BPC_CharacterCustomization_C|SetTargetMesh _bpc_charactercustomization (Variables|Default|GetSkeletalMesh))
  (Variables|/Game/Blueprints/BPC_CharacterCustomization.BPC_CharacterCustomization_C|SetCustomizableComp _bpc_charactercustomization _customizableskeletal)
  (Variables|/Game/Blueprints/BPC_CharacterCustomization.BPC_CharacterCustomization_C|SetCustomizableCompBottom _bpc_charactercustomization _customizableskeletal)
  (Variables|/Game/Blueprints/BPC_CharacterCustomization.BPC_CharacterCustomization_C|SetCustomizableCompTop _bpc_charactercustomization _customizableskeletal)
  (Variables|/Game/Blueprints/BPC_CharacterCustomization.BPC_CharacterCustomization_C|SetCustomizableCompBikiniTop _bpc_charactercustomization _customizableskeletal)
  (Variables|/Game/Blueprints/BPC_CharacterCustomization.BPC_CharacterCustomization_C|SetCustomizableCompBikiniBottom _bpc_charactercustomization _customizableskeletal)
  (Variables|/Game/Blueprints/BPC_CharacterCustomization.BPC_CharacterCustomization_C|SetCustomizableCompHair _bpc_charactercustomization _customizableskeletal)
  (Variables|/Game/Blueprints/BPC_CharacterCustomization.BPC_CharacterCustomization_C|SetHairMesh _bpc_charactercustomization (Variables|Default|GetSkeletalMesh_Hair))
  (Variables|/Game/Blueprints/BPC_CharacterCustomization.BPC_CharacterCustomization_C|SetEyeMeshL _bpc_charactercustomization (Variables|Default|GetSkeletalMesh_EyeL))
  (Variables|/Game/Blueprints/BPC_CharacterCustomization.BPC_CharacterCustomization_C|SetEyeMeshR _bpc_charactercustomization (Variables|Default|GetSkeletalMesh_EyeR))
  (Utilities|Map|Add _clothingmeshes "BikiniTop" (Variables|Default|GetSkeletalMesh_BikiniTop))
  (Utilities|Map|Add _clothingmeshes "TShirt" (Variables|Default|GetSkeletalMesh_Top))
  (Utilities|Map|Add _clothingmeshes "BikiniBottom" (Variables|Default|GetSkeletalMesh_BikiniBottom))
  (Utilities|Map|Add _clothingmeshes "Microshorts" (Variables|Default|GetSkeletalMesh_Bottom))
  (Variables|/Game/Blueprints/BPC_CharacterCustomization.BPC_CharacterCustomization_C|SetPendingUpdates (Variables|Default|GetBPC_CharacterCustomization) 4)
  (Class|CustomizableSkeletalComponent|UpdateSkeletalMeshAsyncResult (Variables|Default|GetCustomizableSkeletal) (EventDispatchers|CreateEvent :!event Custom|OnInitialUpdateFinished) false false)
  (Class|CustomizableSkeletalComponent|UpdateSkeletalMeshAsyncResult (Variables|Default|GetCustomizableSkeletal_Top) (EventDispatchers|CreateEvent :!event Custom|OnInitialUpdateFinished) false false)
  (Class|CustomizableSkeletalComponent|UpdateSkeletalMeshAsyncResult (Variables|Default|GetCustomizableSkeletal_Bottom) (EventDispatchers|CreateEvent :!event Custom|OnInitialUpdateFinished) false false)
  (Class|CustomizableSkeletalComponent|UpdateSkeletalMeshAsyncResult (Variables|Default|GetCustomizableSkeletal_Hair) (EventDispatchers|CreateEvent :!event Custom|OnInitialUpdateFinished) false false)
  (Components|SkinnedMesh|SetLeaderPoseComponent (Variables|Default|GetSkeletalMesh_Top) (Variables|Default|GetSkeletalMesh) false false)
  (Components|SkinnedMesh|SetLeaderPoseComponent (Variables|Default|GetSkeletalMesh_Bottom) (Variables|Default|GetSkeletalMesh) false false)
  (Components|SkinnedMesh|SetLeaderPoseComponent (Variables|Default|GetSkeletalMesh_BikiniBottom) (Variables|Default|GetSkeletalMesh) false false)
  (Components|SkinnedMesh|SetLeaderPoseComponent (Variables|Default|GetSkeletalMesh_BikiniTop) (Variables|Default|GetSkeletalMesh) false false)
  (Components|SkinnedMesh|SetLeaderPoseComponent (Variables|Default|GetSkeletalMesh_EyeL) (Variables|Default|GetSkeletalMesh) false false)
  (Components|SkinnedMesh|SetLeaderPoseComponent (Variables|Default|GetSkeletalMesh_EyeR) (Variables|Default|GetSkeletalMesh) false false)
  (Components|SkinnedMesh|SetLeaderPoseComponent (Variables|Default|GetSkeletalMesh_Hair) (Variables|Default|GetSkeletalMesh) false false)
  (Input|EnableInput (Game|GetPlayerController 0))
  (bind _returnvalue_2 (UserInterface|CreateWidget "/Game/UI/WBP_CharacterCreator.WBP_CharacterCreator_C" 0 (Variables|Default|GetBPC_CharacterCustomization)))
  (UserInterface|Viewport|AddtoViewport _returnvalue_2 0)
  (Transformation|SetRelativeLocation (Variables|Default|GetCameraPivot) "0.000000,0.000000,120.000000" false false)
  (Variables|Default|SetFollowHead false)
  (Variables|Default|SetCameraZOffset 8e+01)
  (Variables|/Script/Engine.SpringArmComponent|SetTargetArmLength (Variables|Default|GetSpringArm) 4e+02)
  (Variables|/Script/Engine.PlayerController|SetbShowMouseCursor _returnvalue true)
  (Game|Player|SetViewTargetwithBlend _returnvalue self 0.0 "VTBlend_Linear" 0.0 false))

(event Collision|EventActorBeginOverlap
  (params (OtherActor :type Actor%20Object%20Reference)))

(event EventTick
  (params (DeltaSeconds :type Float%20%28single-precision%29))
  (Utilities|FlowControl|Sequence
    (:then_0
      (if (Variables|Default|GetbIsRotating)
        (Transformation|AddLocalRotation (Variables|Default|GetCameraPivot) (Math|Rotator|MakeRotator 0.0 0.0 (* (.DeltaX (Class|PlayerController|GetInputMouseDelta (Game|GetPlayerController 0))) (Variables|Default|GetRotationSpeed))) false false)))
    (:then_1
      (bind _value (Default|GetSliderValue (Variables|Default|GetBPC_CharacterCustomization) "height"))
      (Transformation|SetRelativeLocation (Variables|Default|GetSkeletalMesh) (Math|Vector|MakeVector 0.0 0.0 (* _value 14.0)) false false))
    (:then_2
      (if (Variables|Default|GetFollowHead)
        (Transformation|SetRelativeLocation (Variables|Default|GetCameraPivot) (Math|Vector|MakeVector 0.0 0.0 (- (.Z (Math|Vector|BreakVector (Transformation|GetSocketLocation (Variables|Default|GetSkeletalMesh) "Head_M"))) (Variables|Default|GetCameraZOffset))) false false)))))

(event Input|MouseEvents|RightMouseButton
  (params (Key :type Key%20Structure :default "None"))
  (:Pressed
    (Variables|Default|SetbIsRotating true))
  (:Released
    (Variables|Default|SetbIsRotating false)))

(event Input|MouseEvents|MouseWheelUp
  (params (Key :type Key%20Structure :default "None"))
  (bind _springarm (Variables|Default|GetSpringArm))
  (:Pressed
    (Variables|/Script/Engine.SpringArmComponent|SetTargetArmLength _springarm (Math|Float|Clamp(Float) (- (Variables|/Script/Engine.SpringArmComponent|GetTargetArmLength _springarm) (Variables|Default|GetZoomSpeed)) 6e+01 4e+02))))

(event Input|MouseEvents|MouseWheelDown
  (params (Key :type Key%20Structure :default "None"))
  (bind _springarm (Variables|Default|GetSpringArm))
  (:Pressed
    (Variables|/Script/Engine.SpringArmComponent|SetTargetArmLength _springarm (Math|Float|Clamp(Float) (+ (Variables|/Script/Engine.SpringArmComponent|GetTargetArmLength _springarm) (Variables|Default|GetZoomSpeed)) 6e+01 4e+02))))

(event Input|KeyboardEvents|1
  (params (Key :type Key%20Structure :default "None"))
  (:Pressed
    (Variables|Default|SetFollowHead true)
    (Variables|Default|SetCameraZOffset 5.0)
    (Variables|/Script/Engine.SpringArmComponent|SetTargetArmLength (Variables|Default|GetSpringArm) 1e+02)))

(event Input|KeyboardEvents|2
  (params (Key :type Key%20Structure :default "None"))
  (:Pressed
    (Transformation|SetRelativeLocation (Variables|Default|GetCameraPivot) "0.000000,0.000000,100.000000" false false)
    (Variables|Default|SetFollowHead false)
    (Variables|Default|SetCameraZOffset 8e+01)
    (Variables|/Script/Engine.SpringArmComponent|SetTargetArmLength (Variables|Default|GetSpringArm) 6e+02)))

(event Input|KeyboardEvents|Escape
  (params (Key :type Key%20Structure :default "None"))
  (:Pressed
    (Utilities|IsValid (Variables|Default|GetPauseWidget)
      (:Is%20Valid
        (Widget|RemovefromParent (Variables|Default|GetPauseWidget))
        (Variables|Default|SetPauseWidget 0))
      (:Is%20Not%20Valid
        (bind _returnvalue (UserInterface|CreateWidget "/Game/UI/Menu/WBP_PauseMenu.WBP_PauseMenu_C" 0 self))
        (bind _output_get (Variables|Default|SetPauseWidget _returnvalue))
        (UserInterface|Viewport|AddtoViewport _output_get 0)))))

(fn ConstructionScript)

(fn ClearPauseWidget
  (Variables|Default|SetPauseWidget 0))