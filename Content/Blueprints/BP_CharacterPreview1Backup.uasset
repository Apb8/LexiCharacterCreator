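; Character preview actor for the character creator, which opens the creator widget linked to its customization component and becomes the player's view target.
; Holding right mouse yaws the camera pivot, the wheel zooms the spring arm within clamped limits, and keys 1 and 2 switch between close and far framing.
; Every Tick, the "height" slider value is polled from the customization component to offset the skeletal mesh vertically.
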(event EventBeginPlay
  (bind _returnvalue (Game|GetPlayerController 0))
  (Input|EnableInput (Game|GetPlayerController 0))
  (bind _returnvalue_2 (UserInterface|CreateWidget "/Game/UI/WBP_CharacterCreator.WBP_CharacterCreator_C" 0 (Variables|Default|GetBPC_CharacterCustomization)))
  (UserInterface|Viewport|AddtoViewport _returnvalue_2 0)
  (Variables|/Script/Engine.PlayerController|SetbShowMouseCursor _returnvalue true)
  (Game|Player|SetViewTargetwithBlend _returnvalue self 0.5 "VTBlend_Linear" 0.0 false))

(event Collision|EventActorBeginOverlap
  (params (OtherActor :type Actor%20Object%20Reference)))

(event EventTick
  (params (DeltaSeconds :type Float%20%28single-precision%29))
  (Utilities|FlowControl|Sequence
    (:then_0
      (if (Variables|Default|GetbIsRotating)
        (Transformation|AddLocalRotation (Variables|Default|GetCameraPivot) (Math|Rotator|MakeRotator 0.0 0.0 (* (.DeltaX (Class|PlayerController|GetInputMouseDelta (Game|GetPlayerController 0))) (Variables|Default|GetRotationSpeed))) false false)))
    (:then_1
      (bind _value (Default|GetSliderValue (Variables|Default|GetBPC_CharacterCustomization) "height"))
      (Transformation|SetRelativeLocation (Variables|Default|GetSkeletalMesh) (Math|Vector|MakeVector 0.0 0.0 (* _value 14.0)) false false))))

(event Input|MouseEvents|RightMouseButton
  (params (Key :type Key%20Structure))
  (:Pressed
    (Variables|Default|SetbIsRotating true))
  (:Released
    (Variables|Default|SetbIsRotating false)))

(event Input|MouseEvents|MouseWheelUp
  (params (Key :type Key%20Structure))
  (bind _springarm (Variables|Default|GetSpringArm))
  (:Pressed
    (Variables|/Script/Engine.SpringArmComponent|SetTargetArmLength _springarm (Math|Float|Clamp(Float) (- (Variables|/Script/Engine.SpringArmComponent|GetTargetArmLength _springarm) (Variables|Default|GetZoomSpeed)) 6e+01 4e+02))))

(event Input|MouseEvents|MouseWheelDown
  (params (Key :type Key%20Structure))
  (bind _springarm (Variables|Default|GetSpringArm))
  (:Pressed
    (Variables|/Script/Engine.SpringArmComponent|SetTargetArmLength _springarm (Math|Float|Clamp(Float) (+ (Variables|/Script/Engine.SpringArmComponent|GetTargetArmLength _springarm) (Variables|Default|GetZoomSpeed)) 6e+01 4e+02))))

(event Input|KeyboardEvents|1
  (params (Key :type Key%20Structure))
  (:Pressed
    (Transformation|SetRelativeLocation (Variables|Default|GetCameraPivot) "0.000000,0.000000,160.000000" false false)
    (Variables|/Script/Engine.SpringArmComponent|SetTargetArmLength (Variables|Default|GetSpringArm) 1e+02)))

(event Input|KeyboardEvents|2
  (params (Key :type Key%20Structure))
  (:Pressed
    (Transformation|SetRelativeLocation (Variables|Default|GetCameraPivot) "0.000000,0.000000,100.000000" false false)
    (Variables|/Script/Engine.SpringArmComponent|SetTargetArmLength (Variables|Default|GetSpringArm) 6e+02)))

(fn ConstructionScript)