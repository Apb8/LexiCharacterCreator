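; Character customization component that drives face/body morph sliders, makeup, hair and clothing on its owner.
; Data-driven sliders map signed values onto positive/negative morph target pairs.
; Clothing and hair options set Mutable Customizable Object parameters and trigger async mesh updates.
; Makeup, hair and clothing colors go to dynamic materials and are cached, so ReapplyMaterials can rebuild them after a fixed delay following each mesh swap.
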(event Custom|ReapplyMaterials
  (Utilities|FlowControl|Delay 0.5)
  (CallFunction|InitSkinMaterial)
  (bind (_keypin _valuepin) (Utilities|Map|ForEachLoop(Map) (Variables|Default|GetMakeupState))
    (:then
      (CallFunction|SetMakeupTexture _keypin (.Texture (Utilities|Struct|BreakF_MakeupValue _valuepin)))
      (CallFunction|SetMakeupColor _keypin (.Color (Utilities|Struct|BreakF_MakeupValue _valuepin)))
      (CallFunction|SetMakeupIntensity _keypin (.Intensity (Utilities|Struct|BreakF_MakeupValue _valuepin)))
      (CallFunction|InitHairMaterial)
      (CallFunction|SetHairColor (Variables|Default|GetHairColorState))
      (CallFunction|InitClothingMaterials)
      (bind (_keypin_2 _valuepin_2) (Utilities|Map|ForEachLoop(Map) (Variables|Default|GetClothingColors))
        (:then
          (CallFunction|SetClothingColor _keypin_2 _valuepin_2))))))

(event EventBeginPlay
  (bind _morphvalues (Variables|Default|GetMorphValues))
  (Variables|Default|SetTargetMesh (Actor|GetComponentbyClass (Components|GetOwner) "/Script/Engine.SkeletalMeshComponent"))
  (Utilities|Array|Clear _morphvalues)
  (for _array_element (Variables|/Game/Data/BP_MorphSliderData.BP_MorphSliderData_C|GetSliders (Variables|Default|GetSliderData))
    (Utilities|Array|Add _morphvalues (Utilities|Struct|MakeF_MorphValue (.SliderID (Utilities|Struct|BreakF_MorphSliderDef _array_element)) (.DefaultValue (Utilities|Struct|BreakF_MorphSliderDef _array_element))))))

(event EventTick
  (params (DeltaSeconds :type Float%20%28single-precision%29)))

(fn ApplyMorphValue
  (params (SliderID :type Name) (Value :type Float%20%28double-precision%29))
  (bind _targetmesh (Variables|Default|GetTargetMesh))
  (for _array_element (Variables|/Game/Data/BP_MorphSliderData.BP_MorphSliderData_C|GetSliders (Variables|Default|GetSliderData))
    (if (== (.SliderID (Utilities|Struct|BreakF_MorphSliderDef _array_element)) SliderID)
      (if (Utilities|Enum|Equal(Enum) (.SliderType (Utilities|Struct|BreakF_MorphSliderDef _array_element)) "NewEnumerator0")
        (Components|SkeletalMesh|SetMorphTarget _targetmesh (.MorphPositive (Utilities|Struct|BreakF_MorphSliderDef _array_element)) (Math|Float|Max(Float) Value 0.0) true)
        (Components|SkeletalMesh|SetMorphTarget _targetmesh (.MorphNegative (Utilities|Struct|BreakF_MorphSliderDef _array_element)) (Math|Float|Absolute(Float) (Math|Float|Min(Float) Value 0.0)) true)))))

(fn SetSliderValue
  (params (SliderID :type Name) (Value :type Float%20%28double-precision%29))
  (bind _morphvalues (Variables|Default|GetMorphValues))
  (LocalVariables|SetbFound false)
  (for (_array_element _array_index) _morphvalues
    ;[0.15 0.15 0.15 0.5] Add New Value
    (if (== (.SliderID (Utilities|Struct|BreakF_MorphValue _array_element)) SliderID)
      ;[0.15 0.15 0.15 0.5] Update existing value
      (Utilities|Array|SetArrayElem _morphvalues _array_index (Utilities|Struct|MakeF_MorphValue SliderID Value))
      (LocalVariables|SetbFound true)))
  (if (LocalVariables|GetbFound)
    _
    (else
      (Utilities|Array|Add _morphvalues (Utilities|Struct|MakeF_MorphValue SliderID Value))))
  (CallFunction|ApplyMorphValue SliderID Value))

(fn GetSliderValue
  (params (SliderID :type Name))
  (for _array_element (Variables|Default|GetMorphValues)
    (if (== SliderID (.SliderID (Utilities|Struct|BreakF_MorphValue _array_element)))
      (return (.Value (Utilities|Struct|BreakF_MorphValue _array_element)))))
  (return 0.0))

(fn SetClothing
  (params (GroupName :type Name) (OptionName :type Name))
  (Class|CustomizableObjectInstance|SetIntParameterSelectedOption (Class|CustomizableSkeletalComponent|GetCustomizableObjectInstance (Variables|Default|GetCustomizableComp)) (Utilities|String|ToString(Name) GroupName) (Utilities|String|ToString(Name) OptionName) -1)
  (Class|CustomizableSkeletalComponent|UpdateSkeletalMeshAsync (Variables|Default|GetCustomizableComp) false)
  (Class|CustomizableSkeletalComponent|UpdateSkeletalMeshAsync (Variables|Default|GetCustomizableCompTop) false)
  (Class|CustomizableSkeletalComponent|UpdateSkeletalMeshAsync (Variables|Default|GetCustomizableCompBottom) false)
  (Class|CustomizableSkeletalComponent|UpdateSkeletalMeshAsync (Variables|Default|GetCustomizableCompBikiniTop) false)
  (Class|CustomizableSkeletalComponent|UpdateSkeletalMeshAsync (Variables|Default|GetCustomizableCompBikiniBottom) false)
  (CallFunction|ReapplyMaterials))

(fn InitSkinMaterial
  (bind _returnvalue (Rendering|Material|CreateDynamicMaterialInstance (Variables|Default|GetTargetMesh) 0 0 "None" :!class /Script/Engine.PrimitiveComponent))
  (Variables|Default|SetDMI_Skin _returnvalue))

(fn SetMakeupTexture
  (params (Category :type E_MakeupCategory%20Enum :default "NewEnumerator0") (NewTexture :type Texture%202D%20Object%20Reference))
  (bind _dmi_skin (Variables|Default|GetDMI_Skin))
  (bind _makeupparams (Variables|Default|GetMakeupParams))
  (bind _makeupstate (Variables|Default|GetMakeupState))
  (bind _value (Utilities|Map|Find _makeupstate Category))
  (bind (_value_2 _returnvalue) (Utilities|Map|Find _makeupparams Category))
  (bind (_texture _color _intensity) (Utilities|Struct|BreakF_MakeupValue _value))
  (Utilities|IsValid _dmi_skin
    (:Is%20Valid
      (if _returnvalue
        (Rendering|Material|SetTextureParameterValue _dmi_skin (.MaskParam (Utilities|Struct|BreakF_MakeupParamNames _value_2)) NewTexture)
        (Utilities|Map|Add (Variables|Default|GetMakeupState) Category (Utilities|Struct|MakeF_MakeupValue NewTexture _color _intensity))))))

(fn SetMakeupColor
  (params (Category :type E_MakeupCategory%20Enum :default "NewEnumerator0") (NewColor :type Linear%20Color%20Structure))
  (bind _dmi_skin (Variables|Default|GetDMI_Skin))
  (bind _makeupparams (Variables|Default|GetMakeupParams))
  (bind _makeupstate (Variables|Default|GetMakeupState))
  (bind (_value _returnvalue) (Utilities|Map|Find _makeupparams Category))
  (bind _value_2 (Utilities|Map|Find _makeupstate Category))
  (bind (_texture _color _intensity) (Utilities|Struct|BreakF_MakeupValue _value_2))
  (Utilities|IsValid _dmi_skin
    (:Is%20Valid
      (if _returnvalue
        (Rendering|Material|SetVectorParameterValue _dmi_skin (.ColorParam (Utilities|Struct|BreakF_MakeupParamNames _value)) NewColor :!class /Script/Engine.MaterialInstanceDynamic)
        (Utilities|Map|Add (Variables|Default|GetMakeupState) Category (Utilities|Struct|MakeF_MakeupValue _texture NewColor _intensity))))))

(fn SetMakeupIntensity
  (params (Category :type E_MakeupCategory%20Enum :default "NewEnumerator0") (NewIntensity :type Float%20%28double-precision%29))
  (bind _dmi_skin (Variables|Default|GetDMI_Skin))
  (bind _makeupparams (Variables|Default|GetMakeupParams))
  (bind _makeupstate (Variables|Default|GetMakeupState))
  (bind (_value _returnvalue) (Utilities|Map|Find _makeupparams Category))
  (bind _value_2 (Utilities|Map|Find _makeupstate Category))
  (bind (_texture _color) (Utilities|Struct|BreakF_MakeupValue _value_2))
  (Utilities|IsValid _dmi_skin
    (:Is%20Valid
      (if _returnvalue
        (Rendering|Material|SetScalarParameterValue _dmi_skin (.IntensityParam (Utilities|Struct|BreakF_MakeupParamNames _value)) NewIntensity :!class /Script/Engine.MaterialInstanceDynamic)
        (Utilities|Map|Add (Variables|Default|GetMakeupState) Category (Utilities|Struct|MakeF_MakeupValue _texture _color NewIntensity))))))

(fn SetHair
  (params (HairOptionName :type Name))
  (Class|CustomizableObjectInstance|SetIntParameterSelectedOption (Class|CustomizableSkeletalComponent|GetCustomizableObjectInstance (Variables|Default|GetCustomizableComp)) (Utilities|String|ToString(Name) "Hair") (Utilities|String|ToString(Name) HairOptionName) -1)
  (Class|CustomizableSkeletalComponent|UpdateSkeletalMeshAsync (Variables|Default|GetCustomizableCompHair) false)
  (CallFunction|ReapplyMaterials))

(fn InitHairMaterial
  (bind _returnvalue (Rendering|Material|CreateDynamicMaterialInstance (Variables|Default|GetHairMesh) 0 0 "None" :!class /Script/Engine.PrimitiveComponent))
  (Variables|Default|SetDMI_Hair _returnvalue))

(fn SetHairColor
  (params (NewColor :type Linear%20Color%20Structure))
  (bind _dmi_hair (Variables|Default|GetDMI_Hair))
  (Utilities|IsValid _dmi_hair
    (:Is%20Valid
      (Rendering|Material|SetVectorParameterValue _dmi_hair "HairColor" NewColor :!class /Script/Engine.MaterialInstanceDynamic)
      (Variables|Default|SetHairColorState NewColor))))

(fn InitClothingMaterials
  (bind (_keypin _valuepin) (Utilities|Map|ForEachLoop(Map) (Variables|Default|GetClothingMeshes))
    (:then
      (bind _returnvalue (Rendering|Material|CreateDynamicMaterialInstance _valuepin 0 0 "None" :!class /Script/Engine.PrimitiveComponent))
      (Utilities|Map|Add (Variables|Default|GetClothingDMIs) _keypin _returnvalue))))

(fn SetClothingColor
  (params (ClothingID :type Name) (NewColor :type Linear%20Color%20Structure))
  (bind _clothingdmis (Variables|Default|GetClothingDMIs))
  (bind (_value _returnvalue) (Utilities|Map|Find _clothingdmis ClothingID))
  (if _returnvalue
    (Utilities|IsValid _value
      (:Is%20Valid
        (Rendering|Material|SetVectorParameterValue _value "TintColor" NewColor :!class /Script/Engine.MaterialInstanceDynamic)
        (Utilities|Map|Add (Variables|Default|GetClothingColors) ClothingID NewColor)))))